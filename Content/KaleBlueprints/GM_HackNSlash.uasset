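; Game mode for a local multiplayer hack-and-slash that sets up players and handles their character spawning.
; BeginPlay takes the character class from the game instance, defaulting to BP_WaterSpirit, then creates capped local players from PlayerStarts with Enhanced Input mappings.
; Spawn and despawn events replace the pawn with that class or BP_InitialPawn at a random start, keeping the view on GameCamera.
; The options-string pawn selection in GetDefaultPawnClassForController is disconnected.
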(event Custom|SpawnCharacter
  (params (PlayerController :type Player%20Controller%20Object%20Reference))
  (bind _returnvalue (Pawn|GetControlledPawn PlayerController))
  (bind _spawnpoints (Variables|Default|GetSpawnPoints))
  (Utilities|IsValid _returnvalue
    (:Is%20Valid
      (Actor|DestroyActor _returnvalue))
    (:Is%20Not%20Valid
      _))
  ;[1 1 0] Class depends on chosen character
  (bind _returnvalue_2 (Game|SpawnActorfromClass (Variables|Default|GetCharacterClass) (Transformation|GetActorTransform (Utilities|Array|Get(acopy) _spawnpoints (Math|Random|RandomIntegerinRange 0 (- (Utilities|Array|Length _spawnpoints) 1)))) "Undefined" "SelectDefaultAtRuntime" 0 0))
  (Pawn|Possess PlayerController _returnvalue_2)
  (Game|Player|SetViewTargetwithBlend PlayerController (Variables|Default|GetGameCamera) 0.0 "VTBlend_Linear" 0.0 false))

(event Custom|DespawnCharacter
  (params (PlayerController :type Player%20Controller%20Object%20Reference))
  (bind _returnvalue (Pawn|GetControlledPawn PlayerController))
  (bind _spawnpoints (Variables|Default|GetSpawnPoints))
  (Utilities|IsValid _returnvalue
    (:Is%20Valid
      (Actor|DestroyActor _returnvalue))
    (:Is%20Not%20Valid
      _))
  (bind _returnvalue_2 (Game|SpawnActorfromClass "/Game/KaleBlueprints/BP_InitialPawn.BP_InitialPawn_C" (Transformation|GetActorTransform (Utilities|Array|Get(acopy) _spawnpoints (Math|Random|RandomIntegerinRange 0 (- (Utilities|Array|Length _spawnpoints) 1)))) "Undefined" "OverrideRootScale" 0 0))
  (Pawn|Possess PlayerController _returnvalue_2)
  (Game|Player|SetViewTargetwithBlend PlayerController (Variables|Default|GetGameCamera) 0.0 "VTBlend_Linear" 0.0 false))

(event EventBeginPlay
  (Utilities|FlowControl|Sequence
    (:then_0
      (bind _asgi_hack_nslash (Utilities|Casting|CastToGI_HackNSlash (Game|GetGameInstance)))
      (Variables|Default|SetGameInstanceReference _asgi_hack_nslash)
      (if (Utilities|IsValidClass (Variables|/Game/KaleBlueprints/GI_HackNSlash.GI_HackNSlash_C|GetCharacterClass (Variables|Default|GetGameInstanceReference)))
        (Variables|Default|SetCharacterClass (Variables|/Game/KaleBlueprints/GI_HackNSlash.GI_HackNSlash_C|GetCharacterClass (Variables|Default|GetGameInstanceReference)))
        (else
          (Variables|Default|SetCharacterClass "/Game/KaleBlueprints/BP_WaterSpirit.BP_WaterSpirit_C"))))
    (:then_1
      (bind _outactors (Actor|GetAllActorsOfClass "/Script/Engine.PlayerStart"))
      (bind _output_get (Variables|Default|SetSpawnPoints _outactors))
      (for (_ _array_index) _output_get
        (bind _output_get_2 (Variables|Default|SetPlayerIndex _array_index))
        (while (and (== _output_get_2 (Variables|Default|GetNumberOfPlayers)) (<= (Variables|Default|GetNumberOfPlayers) 3))
          (Variables|Default|SetNumberOfPlayers (+ (Variables|Default|GetNumberOfPlayers) 1))
          (bind _returnvalue (Class|GameplayStatics|CreatePlayer _output_get_2))
          (if (> (Variables|Default|GetPlayerIndex) 0)
            (Input|AddMappingContext (PlayerController|LocalPlayerSubsystems|GetEnhancedInputLocalPlayerSubsystem _returnvalue) "/Game/KaleInputs/IMC_StandardGameplay.IMC_StandardGameplay" 0 "(bIgnoreAllPressedKeysUntilRelease=True,bForceImmediately=False)")
            (else
              (Input|AddMappingContext (PlayerController|LocalPlayerSubsystems|GetEnhancedInputLocalPlayerSubsystem (Game|GetPlayerController 0)) "/Game/KaleInputs/IMC_StandardGameplay.IMC_StandardGameplay" 0 "(bIgnoreAllPressedKeysUntilRelease=True,bForceImmediately=False)"))))))))

(event EventTick
  (params (DeltaSeconds :type Float%20%28single-precision%29)))

(fn ConstructionScript)

(fn GetDefaultPawnClassforController
  (params (InController :type Controller%20Object%20Reference)))