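; Player controller for the hack-and-slash mode that lets a player spawn or despawn their character from a gamepad.
; BeginPlay casts the game mode to GM_HackNSlash, caches the reference and prints a confirmation.
; Gamepad Special Right and Special Left call the game mode's SpawnCharacter and DespawnCharacter, passing this controller, so the game mode handles the actual spawning and removal.
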(event EventBeginPlay
  (bind _asgm_hack_nslash (Utilities|Casting|CastToGM_HackNSlash (Game|GetGameMode)))
  (Variables|Default|SetGameModeReference _asgm_hack_nslash)
  (Development|PrintString "Reference Set"))

(event EventTick
  (params (DeltaSeconds :type Float%20%28single-precision%29)))

(event Input|GamepadEvents|GamepadSpecialRight
  (params (Key :type Key%20Structure :default "None"))
  (:Pressed
    (Default|SpawnCharacter (Variables|Default|GetGameModeReference) self)))

(event Input|GamepadEvents|GamepadSpecialLeft
  (params (Key :type Key%20Structure :default "None"))
  (:Pressed
    (Default|DespawnCharacter (Variables|Default|GetGameModeReference) self)))

(fn ConstructionScript)